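; BP_EnemyUsingLerp is an enemy actor that moves and rotates on timelines and damages whatever it hits.
; On BeginPlay, the movement timeline, paced by MovementSpeed, lerps location between minimum and maximum offsets from the start position.
; A parallel rotation timeline lerps from the initial rotation to a target scaled from RotationSpeed.
; Hit events apply Damage to the other actor, and the F key prints a debug string.
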(event EventBeginPlay
  (Utilities|FlowControl|Sequence
    (:then_0
      ;[1 1 1] Movement Loop
      (Components|Timeline|SetPlayRate (Variables|Default|GetMovement%20Timeline) (Variables|Movement|GetMovement%20Speed))
      (bind _output_get (Variables|Movement|SetInitial%20Location (Transformation|GetActorLocation)))
      (bind _alpha_value (Timeline|Movement%20Timeline Play)
        (:Update
          (Transformation|SetActorLocation (Math|Vector|Lerp(Vector) (+ _output_get (Variables|Movement|GetMin%20Distance)) (+ _output_get (Variables|Movement|GetMax%20Distance)) _alpha_value) false false))))
    (:then_1
      ;[1 1 1] Rotation Loop
      (bind _output_get_2 (Variables|Movement|SetInitial%20Rotation (Transformation|GetActorRotation)))
      (bind _alpha_value_2 (Timeline|Rotation%20Timeline Play)
        (:Update
          (Transformation|SetActorRotation (Math|Rotator|Lerp(Rotator) _output_get_2 (* (Variables|Movement|GetRotation%20Speed) 359.0) _alpha_value_2)))))))

(event Collision|EventHit
  (params (MyComp :type Primitive%20Component%20Object%20Reference) (Other :type Actor%20Object%20Reference) (OtherComp :type Primitive%20Component%20Object%20Reference) (bSelfMoved :type Boolean) (HitLocation :type Vector :default "0, 0, 0") (HitNormal :type Vector :default "0, 0, 0") (NormalImpulse :type Vector :default "0, 0, 0") (Hit :type Hit%20Result%20Structure%20%28by%20ref%29))
  (Game|Damage|ApplyDamage Other (Variables|Default|GetDamage) 0 0))

(event Input|KeyboardEvents|F
  (params (Key :type Key%20Structure :default "None"))
  (:Pressed
    (Development|PrintString "Hello")))

(fn ConstructionScript)