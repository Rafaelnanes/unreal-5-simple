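; Tick-driven enemy hazard that oscillates and spins its cube mesh and applies damage to any actor it hits.
; Each Tick, per-axis helpers step relative location between min/max limits and add rotation speed to roll, pitch and yaw.
; All three movement axes share one RevertMovement direction flag, so a limit on one axis affects the others.
; Speeds apply per frame without delta-time scaling.
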(event EventTick
  (params (DeltaSeconds :type Float%20%28single-precision%29))
  (Utilities|FlowControl|Sequence
    (:then_0
      ;[1 1 1] Movement
      (bind _returnvalue (CallFunction|SetXMovement))
      (Transformation|SetRelativeLocation (Variables|Default|GetSM_Cube) (Math|Vector|MakeVector _returnvalue (stale _returnvalue_2) (stale _returnvalue_3)) false false :!label _label))
    (:then_1
      (bind _returnvalue_2 (CallFunction|SetYMovement))
      (goto _label))
    (:then_2
      (bind _returnvalue_3 (CallFunction|SetZMovement))
      (goto _label))
    (:then_3
      ;[1 1 1] Rotation
      (bind _returnvalue_4 (CallFunction|SetXRotation))
      (Transformation|SetRelativeRotation (Variables|Default|GetSM_Cube) (Math|Rotator|MakeRotator _returnvalue_4 (stale _returnvalue_5) (stale _returnvalue_6)) false false :!label _label_2))
    (:then_4
      (bind _returnvalue_5 (CallFunction|SetYRotation))
      (goto _label_2))
    (:then_5
      (bind _returnvalue_6 (CallFunction|SetZRotation))
      (goto _label_2))))

(event Collision|EventHit
  (params (MyComp :type Primitive%20Component%20Object%20Reference) (Other :type Actor%20Object%20Reference) (OtherComp :type Primitive%20Component%20Object%20Reference) (bSelfMoved :type Boolean) (HitLocation :type Vector :default "0, 0, 0") (HitNormal :type Vector :default "0, 0, 0") (NormalImpulse :type Vector :default "0, 0, 0") (Hit :type Hit%20Result%20Structure%20%28by%20ref%29))
  (Game|Damage|ApplyDamage Other (Variables|Default|GetDamage) 0 0))

(fn ConstructionScript)

(fn CalculateMovement
  (params (ValueReference :type Float%20%28double-precision%29) (MaxLimit :type Float%20%28double-precision%29) (MinLimit :type Float%20%28double-precision%29) (Speed :type Float%20%28double-precision%29))
  (if (> ValueReference MaxLimit)
    (Variables|Movement|SetRevertMovement true)
    (elif (< ValueReference MinLimit)
      (Variables|Movement|SetRevertMovement false)))
  (return (select (Variables|Movement|GetRevertMovement) (- ValueReference Speed) (+ ValueReference Speed))))

(fn SetXMovement
  ;[1 1 1] Set X
  (bind _returnvalue (CallFunction|CalculateMovement (.x (Variables|/Script/Engine.SceneComponent|GetRelativeLocation (Variables|Default|GetSM_Cube))) (.x (Variables|Movement|GetMaxDistance)) (.x (Variables|Movement|GetMinDistance)) (.x (Variables|Movement|GetMovementSpeed))))
  (return _returnvalue))

(fn SetYMovement
  ;[1 1 1] Set Y
  (bind _returnvalue (CallFunction|CalculateMovement (.y (Variables|/Script/Engine.SceneComponent|GetRelativeLocation (Variables|Default|GetSM_Cube))) (.y (Variables|Movement|GetMaxDistance)) (.y (Variables|Movement|GetMinDistance)) (.y (Variables|Movement|GetMovementSpeed))))
  (return _returnvalue))

(fn SetZMovement
  ;[1 1 1] Set Y
  (bind _returnvalue (CallFunction|CalculateMovement (.z (Variables|/Script/Engine.SceneComponent|GetRelativeLocation (Variables|Default|GetSM_Cube))) (.z (Variables|Movement|GetMaxDistance)) (.z (Variables|Movement|GetMinDistance)) (.z (Variables|Movement|GetMovementSpeed))))
  (return _returnvalue))

(fn SetXRotation
  ;[1 1 1] Set X Rotation
  (bind _returnvalue (CallFunction|CalculateRotation (.roll (Variables|/Script/Engine.SceneComponent|GetRelativeRotation (Variables|Default|GetSM_Cube))) (.x (Variables|Movement|GetRotationSpeed))))
  (return _returnvalue))

(fn CalculateRotation
  (params (ValueReference :type Float%20%28double-precision%29) (Speed :type Float%20%28double-precision%29))
  (return (+ ValueReference Speed)))

(fn SetYRotation
  ;[1 1 1] Set Y Rotation
  (bind _returnvalue (CallFunction|CalculateRotation (.pitch (Variables|/Script/Engine.SceneComponent|GetRelativeRotation (Variables|Default|GetSM_Cube))) (.y (Variables|Movement|GetRotationSpeed))))
  (return _returnvalue))

(fn SetZRotation
  ;[1 1 1] Set Z Rotation
  (bind _returnvalue (CallFunction|CalculateRotation (.yaw (Variables|/Script/Engine.SceneComponent|GetRelativeRotation (Variables|Default|GetSM_Cube))) (.z (Variables|Movement|GetRotationSpeed))))
  (return _returnvalue))