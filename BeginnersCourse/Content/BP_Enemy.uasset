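; BP_Enemy is an enemy Blueprint whose Cube component patrols back and forth and spins every frame.
; Tick sequences per-axis helpers into shared SetRelativeLocation and SetRelativeRotation calls, each fired three times per frame.
; CalculateMovement steps between MinDistance and MaxDistance using one RevertMovement flag shared by all axes, while CalculateRotation simply adds RotationSpeed.
; Both steps ignore delta time, so motion depends on frame rate.
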(event EventTick
  (params (DeltaSeconds :type Float%20%28single-precision%29))
  (Utilities|FlowControl|Sequence
    (:then_0
      ;[1 1 1] Movement
      (bind _returnvalue (CallFunction|SetXMovement))
      (Transformation|SetRelativeLocation (Variables|Default|GetCube) (Math|Vector|MakeVector _returnvalue (stale _returnvalue_2) (stale _returnvalue_3)) false false :!label _label))
    (:then_1
      (bind _returnvalue_2 (CallFunction|SetYMovement))
      (goto _label))
    (:then_2
      (bind _returnvalue_3 (CallFunction|SetZMovement))
      (goto _label))
    (:then_3
      ;[1 1 1] Rotation
      (bind _returnvalue_4 (CallFunction|SetXRotation))
      (Transformation|SetRelativeRotation (Variables|Default|GetCube) (Math|Rotator|MakeRotator _returnvalue_4 (stale _returnvalue_5) (stale _returnvalue_6)) false false :!label _label_2))
    (:then_4
      (bind _returnvalue_5 (CallFunction|SetYRotation))
      (goto _label_2))
    (:then_5
      (bind _returnvalue_6 (CallFunction|SetZRotation))
      (goto _label_2))))

(fn ConstructionScript)

(fn CalculateMovement
  (params (ValueReference :type Float%20%28double-precision%29) (MaxLimit :type Float%20%28double-precision%29) (MinLimit :type Float%20%28double-precision%29) (Speed :type Float%20%28double-precision%29))
  (if (> ValueReference MaxLimit)
    (Variables|Default|SetRevertMovement true)
    (elif (< ValueReference MinLimit)
      (Variables|Default|SetRevertMovement false)))
  (return (select (Variables|Default|GetRevertMovement) (- ValueReference Speed) (+ ValueReference Speed))))

(fn SetXMovement
  ;[1 1 1] Set X
  (bind _returnvalue (CallFunction|CalculateMovement (.x (Variables|/Script/Engine.SceneComponent|GetRelativeLocation (Variables|Default|GetCube))) (.x (Variables|Default|GetMaxDistance)) (.x (Variables|Default|GetMinDistance)) (.x (Variables|Default|GetMovementSpeed))))
  (return _returnvalue))

(fn SetYMovement
  ;[1 1 1] Set Y
  (bind _returnvalue (CallFunction|CalculateMovement (.y (Variables|/Script/Engine.SceneComponent|GetRelativeLocation (Variables|Default|GetCube))) (.y (Variables|Default|GetMaxDistance)) (.y (Variables|Default|GetMinDistance)) (.y (Variables|Default|GetMovementSpeed))))
  (return _returnvalue))

(fn SetZMovement
  ;[1 1 1] Set Y
  (bind _returnvalue (CallFunction|CalculateMovement (.z (Variables|/Script/Engine.SceneComponent|GetRelativeLocation (Variables|Default|GetCube))) (.z (Variables|Default|GetMaxDistance)) (.z (Variables|Default|GetMinDistance)) (.z (Variables|Default|GetMovementSpeed))))
  (return _returnvalue))

(fn SetXRotation
  ;[1 1 1] Set X Rotation
  (bind _returnvalue (CallFunction|CalculateRotation (.roll (Variables|/Script/Engine.SceneComponent|GetRelativeRotation (Variables|Default|GetCube))) (.x (Variables|Default|GetRotationSpeed))))
  (return _returnvalue))

(fn CalculateRotation
  (params (ValueReference :type Float%20%28double-precision%29) (Speed :type Float%20%28double-precision%29))
  (return (+ ValueReference Speed)))

(fn SetYRotation
  ;[1 1 1] Set Y Rotation
  (bind _returnvalue (CallFunction|CalculateRotation (.pitch (Variables|/Script/Engine.SceneComponent|GetRelativeRotation (Variables|Default|GetCube))) (.y (Variables|Default|GetRotationSpeed))))
  (return _returnvalue))

(fn SetZRotation
  ;[1 1 1] Set Z Rotation
  (bind _returnvalue (CallFunction|CalculateRotation (.yaw (Variables|/Script/Engine.SceneComponent|GetRelativeRotation (Variables|Default|GetCube))) (.z (Variables|Default|GetRotationSpeed))))
  (return _returnvalue))