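; BP_Door is an interactable door that the player can open only after collecting all orbs.
; Overlapping its collision box enables input, shows either a press-F or collect-more-orbs prompt, and opens a Gate only if BP_Player reports having all orbs.
; The item action passes through that Gate to a FlipFlop that plays or reverses a timeline driving the mesh's yaw.
; Leaving the box disables input, closes the Gate, reverses the rotation and hides both prompts.
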(event OnComponentBeginOverlap(CollisionBox)
  (params (OverlappedComponent :type Primitive%20Component%20Object%20Reference) (OtherActor :type Actor%20Object%20Reference) (OtherComp :type Primitive%20Component%20Object%20Reference) (OtherBodyIndex :type Integer) (bFromSweep :type Boolean) (SweepResult :type Hit%20Result%20Structure%20%28by%20ref%29))
  (bind _staticmesh (Variables|Default|GetStaticMesh))
  (bind _returnvalue (Transformation|GetRelativeTransform _staticmesh))
  ;[1 1 1] Open
  (bind _asbp_player (Utilities|Casting|CastToBP_Player OtherActor))
  (Variables|Default|SetPlayer _asbp_player)
  (Input|EnableInput (Game|GetPlayerController 0))
  (if (Default|HasAllOrbs (Variables|Default|GetPlayer))
    (CallFunction|SetTextVisibility)
    (Utilities|FlowControl|Gate true) ; enters at Open
    (else
      (CallFunction|SetTextVisibility))))

(event OnComponentEndOverlap(CollisionBox)
  (params (OverlappedComponent :type Primitive%20Component%20Object%20Reference) (OtherActor :type Actor%20Object%20Reference) (OtherComp :type Primitive%20Component%20Object%20Reference) (OtherBodyIndex :type Integer))
  (bind _staticmesh (Variables|Default|GetStaticMesh))
  (bind _returnvalue (Transformation|GetRelativeTransform _staticmesh))
  ;[1 1 1] Close
  (Utilities|Casting|CastToBP_Player OtherActor)
  (Input|DisableInput (Game|GetPlayerController 0))
  (Utilities|FlowControl|Sequence
    (:then_0
      (Utilities|FlowControl|Gate true) ; enters at Close
    )
    (:then_1
      (bind _movementtime (Timeline|Rotate Reverse)
        (:Update
          ;[1 1 1] Change Door Rotation
          (Transformation|SetRelativeRotation (Variables|Default|GetStaticMesh) (Math|Rotator|MakeRotator (.roll (.rotation _returnvalue)) (.pitch (.rotation _returnvalue)) _movementtime) false false))))
    (:then_2
      (Rendering|SetVisibility (Variables|Default|GetPressFText) false false)
      (Rendering|SetVisibility (Variables|Default|GetCollect%20More%20Orbs) false false))))

(event Input|EnhancedActionEvents|EnhancedInputActionIA_ItemAction
  (params (ActionValue :type Boolean) (ElapsedSeconds :type Float%20%28double-precision%29) (TriggeredSeconds :type Float%20%28double-precision%29) (InputAction :type Input%20Action%20Object%20Reference :default "/Game/Player/Controller/IA_ItemAction.IA_ItemAction"))
  (bind _staticmesh (Variables|Default|GetStaticMesh))
  (bind _returnvalue (Transformation|GetRelativeTransform _staticmesh))
  (Utilities|FlowControl|Gate true
    (:Exit
      (Utilities|FlowControl|FlipFlop
        (:A
          (bind _movementtime (Timeline|Rotate PlayFromStart)
            (:Update
              ;[1 1 1] Change Door Rotation
              (Transformation|SetRelativeRotation (Variables|Default|GetStaticMesh) (Math|Rotator|MakeRotator (.roll (.rotation _returnvalue)) (.pitch (.rotation _returnvalue)) _movementtime) false false))))
        (:B
          (Timeline|Rotate Reverse))))))

(fn ConstructionScript)

(fn SetTextVisibility
  (bind _collect_more_orbs (Variables|Default|GetCollect%20More%20Orbs))
  (if (Default|HasAllOrbs (Variables|Default|GetPlayer))
    (Rendering|SetVisibility (Variables|Default|GetPressFText) true false)
    (Rendering|SetVisibility _collect_more_orbs false false)
    (else
      (Rendering|SetVisibility (Variables|Default|GetPressFText) false false)
      (Rendering|SetVisibility _collect_more_orbs true false))))